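; Mars game mode that runs successive waves of BP_Spider enemies, with wave size computed by a math expression from the incrementing wave count.
; On BeginPlay it gathers all TargetPoints as spawn points, then starts the first wave.
; Each wave spawns spiders at those points in randomly delayed rounds, gated by ShouldSpawn, until its budget is spent.
; OnEnemyKilled removes the spider and starts another wave shortly after the tracked list empties.
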(event Custom|Event%20StartWave
  (bind _spawnrounddelay (Variables|EnemySpawning|GetSpawnRoundDelay))
  (bind (_x _y) (Math|Vector2D|BreakVector2D _spawnrounddelay))
  (EnemySpawning|StartWave)
  (while (EnemySpawning|AreEnemiesSpawning)
    (EnemySpawning|SpawnEnemies)
    (Utilities|FlowControl|Delay (Math|Random|RandomFloatinRange _x _y))))

(event Custom|Event%20OnEnemyKilled
  (params (Enemy :type Object%20Object%20Reference))
  (bind _asbp_spider (Utilities|Casting|CastToBP_Spider Enemy))
  (bind _remaining (|RemoveEnemy _asbp_spider))
  (if (<= _remaining 0)
    (Utilities|FlowControl|Delay 2.0)
    (CallFunction|EventStartWave)))

(event EventBeginPlay
  (Utilities|FlowControl|DelayUntilNextTick)
  (CallFunction|Initialize)
  (Utilities|FlowControl|Delay 2.0)
  (CallFunction|EventStartWave))

(event EventTick
  (params (DeltaSeconds :type Float%20%28single-precision%29)))

(fn ConstructionScript)

(fn AreEnemiesSpawning
  (return (> (Variables|EnemySpawning|GetWaveRemaining) 0)))

(fn AreEnemiesAlive
  (return (> (Utilities|Array|Length (Variables|EnemySpawning|GetEnemies)) 0)))

(fn StartWave
  (Math|Integer|IncrementInt (Variables|EnemySpawning|GetWaveCount)
    (:%20%20
      (bind _output_get (Variables|EnemySpawning|SetWaveSize (Math|Float|Truncate (|(({7BBC0299-6140-0C24-ACC3-6D99FE88F803}*(pow({D63F771D-B54E-6124-3E7B-57B59D7404C7},{7AE248EF-0847-FF23-A331-C38B6C100FF4})))+{5DBA8142-F148-29EB-18F4-9D88AAD9B660})))))
      (Variables|EnemySpawning|SetWaveRemaining _output_get))))

(fn Initialize
  (bind _outactors (Actor|GetAllActorsOfClass "/Script/Engine.TargetPoint"))
  (Variables|EnemySpawning|SetEnemySpawnPoints _outactors))

(fn SpawnEnemies
  (for _array_element (Variables|EnemySpawning|GetEnemySpawnPoints)
    (if (|ShouldSpawn)
      (EnemySpawning|SpawnEnemy (Transformation|GetActorTransform _array_element)))))

(fn SpawnEnemy
  (params (SpawnTransform :type Transform))
  (bind _returnvalue (Game|SpawnActorfromClass "/Game/Blueprint/Pawns/BP_Spider.BP_Spider_C" SpawnTransform "Undefined" "MultiplyWithRoot" 0 0))
  (Math|Integer|DecrementInt (Variables|EnemySpawning|GetWaveRemaining)
    (:%20%20
      (Utilities|Array|Add (Variables|EnemySpawning|GetEnemies) _returnvalue))))