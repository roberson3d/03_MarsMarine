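; Spider enemy character that chases player 0 with a repeating AI MoveTo, retried a second after each success or failure while it is alive.
; Tick starts an attack montage when a living marine player is in range, pausing movement until it completes; a separate DamagePlayer function applies the hit.
; Damage reduces health; on death it stops, notifies the killing marine and Mars game mode, then destroys itself after a delay.
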(event EventBeginPlay
  (CallFunction|InitializeSpider)
  (if (TakeDamage|IsAlive) :!label _label
    (AI|AIMoveTo self "0, 0, 0" (Game|GetPlayerCharacter 0) 5.0 false
      (:OnSuccess
        _)
      (:OnFail
        _))
    (Utilities|FlowControl|Delay 1.0)
    (goto _label)))

(event Collision|EventActorBeginOverlap
  (params (OtherActor :type Actor%20Object%20Reference)))

(event EventTick
  (params (DeltaSeconds :type Float%20%28single-precision%29))
  (if (Attacking|CanAttack)
    (|Attack)))

(event Game|Damage|EventAnyDamage
  (params (Damage :type Float%20%28single-precision%29) (DamageType :type Damage%20Type%20Object%20Reference) (InstigatedBy :type Controller%20Object%20Reference) (DamageCauser :type Actor%20Object%20Reference))
  (if (not (Variables|Default|GetIsDead))
    (TakeDamage|DecrementHealth Damage InstigatedBy)
    (if (Variables|Default|GetIsDead)
      (Movement|DeactivateAIMovement)
      (TakeDamage|NotifyOthersOfDeath InstigatedBy)
      (Utilities|FlowControl|Delay 2.5)
      (TakeDamage|Kill))))

(fn ConstructionScript)

(fn ActivateAIMovement
  (Components|Activation|Activate (Variables|Character|GetCharacterMovement) false))

(fn DeactivateAIMovement
  (bind _charactermovement (Variables|Character|GetCharacterMovement))
  (Components|Movement|StopMovementImmediately _charactermovement)
  (Components|Activation|Deactivate _charactermovement))

(fn IsAttacking
  (return (Animation|Montage|MontageIsPlaying (Components|SkeletalMesh|GetAnimInstance (Variables|Character|GetMesh)) "/Game/Characters/Enemy_Great_Spider/Animations/AniMt_SpiderAttack.AniMt_SpiderAttack")))

(fn IsWithinAttackRange
  (return (<= (Transformation|GetDistanceTo (Game|GetPlayerCharacter 0)) (Variables|Default|GetAttackRange))))

(fn HasValidTarget
  (bind _asbp_marine (Utilities|Casting|CastToBP_Marine (Game|GetPlayerCharacter 0)))
  (return (Default|IsAlive _asbp_marine)))

(fn CanAttack
  (return (Math|Boolean|ANDBoolean (TakeDamage|IsAlive) (not (Attacking|IsAttacking)) (Attacking|HasValidTarget) (Attacking|IsWithinAttackRange))))

(fn DamagePlayer
  (Game|Damage|ApplyDamage (Game|GetPlayerCharacter 0) (Variables|Default|GetAttackDamage) (Pawn|GetController) self))

(fn IsAlive
  (return (not (Variables|Default|GetIsDead))))

(fn DecrementHealth
  (params (Damage :type Float%20%28double-precision%29) (Attacker :type Actor%20Object%20Reference))
  (if (TakeDamage|IsAlive)
    (bind _health (|ReduceHealth Damage))
    (|CheckForDeath _health
      (:then
        _)))
  (return))

(fn InitializeSpider
  (Variables|Default|SetHealth (Variables|Default|GetHealthMax)))

(fn NotifyOthersOfDeath
  (params (Attacker :type Actor%20Object%20Reference))
  (|NotifyKiller Attacker)
  (|NotifyGameMode))

(fn Kill
  (if (Variables|Default|GetIsDead)
    (Actor|DestroyActor)
    (Collision|SetActorEnableCollision false)))